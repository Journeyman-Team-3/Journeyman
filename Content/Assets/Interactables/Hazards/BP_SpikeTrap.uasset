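; BP_SpikeTrap is a hazard whose spikes rise and retract after an overlap with its ActiveArea.
; Delays time the two component moves along the relative Z axis.
; HitZone overlaps damage Entity actors and destroy them when TakeDamage returns false, using a DoOnce reset after a short delay to limit repeated hits.
; EnableTrap and DisableTrap are empty stubs.
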(event `self.HitZone.OnComponentBeginOverlap`
  (params (OverlappedComponent :type "PrimitiveComponent Object Reference") (OtherActor :type "Actor Object Reference") (OtherComp :type "PrimitiveComponent Object Reference") (OtherBodyIndex :type Integer) (bFromSweep :type Boolean) (SweepResult :type "HitResult Structure (by ref)"))
  (bind _temp_actor (`self.Temp Actor`))
  ;[1 1 1] Actor activates trap
  (set `self.Temp Actor` OtherActor)
  (`|ExecutionSequence`
    (:`then_0`
      (`/Engine/EditorBlueprintResources/StandardMacros.DoOnce` false :!label _label ; Trigger box seems to hit actor multiple times
        (:`Completed`
          (`KismetSystemLibrary.PrintString` "Hit by spike")
          (bind _asentity (cast `Entity` _temp_actor))
          (bind _returnvalue (`Entity.TakeDamage` _asentity 10))
          (if _returnvalue
            (`KismetSystemLibrary.PrintString` "hit")
            (else
              (`self.K2_DestroyActor` _temp_actor))))))
    (:`then_1`
      (`KismetSystemLibrary.Delay` 0.2)
      (goto _label :!via `Reset`))))

(event `self.ActiveArea.OnComponentBeginOverlap`
  (params (OverlappedComponent :type "PrimitiveComponent Object Reference") (OtherActor :type "Actor Object Reference") (OtherComp :type "PrimitiveComponent Object Reference") (OtherBodyIndex :type Integer) (bFromSweep :type Boolean) (SweepResult :type "HitResult Structure (by ref)"))
  ;[1 1 1] If actor is hit zone
  (`KismetSystemLibrary.Delay` (`self.DelayActivate`))
  (`KismetSystemLibrary.MoveComponentTo` (`self.Spikes`) (0.0 0.0 30.0)) ; if this was instead an animation, this could be \nplaced on walls aswell or something
  (`KismetSystemLibrary.Delay` (`self.DelayRetract`))
  (`KismetSystemLibrary.MoveComponentTo` (`self.Spikes`) (0.0 0.0 -50.0)) ; for some reason -30 doesnt bring it back down fully\nbut - 50 does
)

(fn `UserConstructionScript`)