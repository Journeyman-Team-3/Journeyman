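; LockOnVisual is an actor that provides Tab-toggled target lock-on with an indicator widget over the nearest candidate.
; Tick scans all actors of a class, stores the one nearest the player within range and moves the widget above it, showing it once locked.
; Tab locks that actor or clears the lock and resets this actor's rotation.
; Leaving range hides the widget and drops the lock.
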(event `Key|Tab`
  (params (Key :type "Key Structure"))
  (:`Pressed`
    (`self.LockTarget`
      (:`then`
        (set `self.LockTarget` null)
        (set `self.IsCloseEnough` false)
        (set `self.NearestEnemy` null)
        (`self.K2_SetActorRotation` (struct)))
      (:`else`
        (if true
          (set `self.LockTarget` (`self.NearestEnemy`)))))))

(event `self.ReceiveTick`
  (params (DeltaSeconds :type "Float (single-precision)"))
  (bind _returnvalue (`self.GetTransform` (`self.NearestEnemy`)))
  (bind _outactors (`GameplayStatics.GetAllActorsOfClass` null)) ; Get all actors in a class (eventually there will be an enemyclass that holds this data)
  (bind (_distance _returnvalue_2) (`GameplayStatics.FindNearestActor` (`self.K2_GetActorLocation` (`GameplayStatics.GetPlayerPawn` 0)) _outactors))
  (if (< _distance 1000.0)
    (set `self.NearestEnemy` _returnvalue_2)
    (`SceneComponent.K2_SetWorldLocation` (`self.LockOnWidget`) (`KismetMathLibrary.MakeVector` (.x (.location _returnvalue)) (.y (.location _returnvalue)) (+ (.z (.location _returnvalue)) 100.0)) false false)
    (set `self.IsCloseEnough` true)
    (`self.LockTarget`
      (:`then`
        (`SceneComponent.SetVisibility` (`self.LockOnWidget`) true false))
      (:`else`))
    (else
      (`SceneComponent.SetVisibility` (`self.LockOnWidget`) false false)
      (set `self.LockTarget` null)
      (set `self.IsCloseEnough` false))))

(fn `UserConstructionScript`)