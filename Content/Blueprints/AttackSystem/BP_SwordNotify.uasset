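; BP_SwordNotify is an animation notify state that marks the window in an animation during which the owner's sword trigger is active.
; On begin and end it looks up BP_AttackComponent on the mesh's owner and calls TriggerSword and StopTriggerSword respectively, returning false if none is found.
; The begin event also prints a debug string.
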(fn `Received_NotifyBegin`
  (params (MeshComp :type "SkeletalMeshComponent Object Reference") (Animation :type "AnimSequenceBase Object Reference") (TotalDuration :type "Float (double-precision)"))
  (returns (ReturnValue :type Boolean))
  (locals (TempAttackComponent :type "AttackComponent Object Reference"))
  (`KismetSystemLibrary.PrintString` null "BLUEPRINT")
  (bind _output_get (set `local.TempAttackComponent` (`Actor.GetComponentByClass` (`ActorComponent.GetOwner` MeshComp) "/Game/Blueprints/AttackSystem/BP_AttackComponent.BP_AttackComponent_C")))
  (if (`KismetSystemLibrary.IsValid` _output_get)
    (bind _asbp_attack_component (cast `/Game/Blueprints/AttackSystem/BP_AttackComponent` (`local.TempAttackComponent`)))
    (`/Game/Blueprints/AttackSystem/BP_AttackComponent.TriggerSword` _asbp_attack_component)
    (return true)
    (else
      (return false))))

(fn `Received_NotifyEnd`
  (params (MeshComp :type "SkeletalMeshComponent Object Reference") (Animation :type "AnimSequenceBase Object Reference"))
  (returns (ReturnValue :type Boolean))
  (locals (TempAttackComponent :type "AttackComponent Object Reference"))
  (bind _output_get (set `local.TempAttackComponent` (`Actor.GetComponentByClass` (`ActorComponent.GetOwner` MeshComp) "/Game/Blueprints/AttackSystem/BP_AttackComponent.BP_AttackComponent_C")))
  (if (`KismetSystemLibrary.IsValid` _output_get)
    (bind _asbp_attack_component (cast `/Game/Blueprints/AttackSystem/BP_AttackComponent` (`local.TempAttackComponent`)))
    (`/Game/Blueprints/AttackSystem/BP_AttackComponent.StopTriggerSword` _asbp_attack_component)
    (return true)
    (else
      (return false))))