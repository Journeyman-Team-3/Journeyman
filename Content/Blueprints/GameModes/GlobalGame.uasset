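; GlobalGame is a shared game-state Blueprint that caches player stats and spawns floating combat text.
; StoreCharacter saves health, stamina and mana, and SetCharacterValues copies them back onto a player unless stored health is zero.
; It also holds a flag for whether the game just began.
; SpawnFloatingCombatText projects a world location to the first player's screen and adds a FloatingDamage widget showing the damage.
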(fn `GetCharacterValues`
  (returns (health :type "Float (double-precision)") (stam :type "Float (double-precision)") (mana :type "Float (double-precision)"))
  (return (`self.player_health`) (`self.player_stam`) (`self.player_mana`)))

(fn `Set Start Bool`
  (params (NewParam :type Boolean))
  (set `self.has_Game_JUST_Begun` NewParam))

(fn `SetCharacterValues`
  (params (`Player In` :type "Entity Object Reference"))
  (if (not (== (`self.player_health`) 0.0))
    (bind (_health _stam _mana) (`self.GetCharacterValues`))
    (set `Entity.health` _health `Player In`)
    (set `Entity.stamina` _stam `Player In`)
    (set `Entity.mana` _mana `Player In`)))

(fn `SpawnFloatingCombatText`
  (params (WorldLocation :type "Vector Structure") (Damage :type "Float (double-precision)"))
  (bind _returnvalue (`GameplayStatics.GetPlayerController` 0))
  (bind _returnvalue_2 (`|CreateWidget` "/Game/UserInterface/FloatingDamage.FloatingDamage_C" _returnvalue (`GameplayStatics.ProjectWorldToScreen` _returnvalue WorldLocation) Damage))
  (`UserWidget.AddToViewport` _returnvalue_2 10))

(fn `StoreCharacter`
  (params (EntityIn :type "Entity Object Reference"))
  (set `self.player_health` (`Entity.health` EntityIn))
  (set `self.player_stam` (`Entity.stamina` EntityIn))
  (set `self.player_mana` (`Entity.mana` EntityIn)))