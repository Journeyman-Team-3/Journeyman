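; Demo weapon Blueprint that deals fixed damage to actors it hits, with a crude one-second hit cooldown.
; A successful TakeDamage sets a shared Hit flag and records the timecode, while debug prints report success or "Dead".
; Later hits only clear the flag once the timecode's seconds field has advanced enough, so that hit deals no damage.
; The single flag prevents damaging several targets at once.
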(event `self.OnHitActor`
  (params (EntityHit :type "Entity Object Reference"))
  (bind (_returnvalue_hours _returnvalue_minutes _returnvalue_seconds) (break `Timecode` (`TimeManagementBlueprintLibrary.GetTimecode`)))
  (bind (_timeathit_hours _timeathit_minutes _timeathit_seconds) (break `Timecode` (`self.timeAtHit`)))
  (if (`self.hit`)
    (if (>= _returnvalue_seconds (+ _timeathit_seconds 1))
      (set `self.hit` false))
    (else
      (bind _returnvalue (`Entity.TakeDamage` EntityHit 10))
      (if _returnvalue
        (set `self.hit` true)
        (set `self.timeAtHit` (`TimeManagementBlueprintLibrary.GetTimecode`))
        (`KismetSystemLibrary.PrintString` "Hello")
        (else
          (`KismetSystemLibrary.PrintString` "Dead"))))))

(fn `UserConstructionScript`)