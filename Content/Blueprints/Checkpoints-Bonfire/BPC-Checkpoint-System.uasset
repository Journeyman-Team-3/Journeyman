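; Checkpoint component for the bonfire system that remembers the selected checkpoint tag and respawns the player there by reloading the level.
; On BeginPlay it binds handlers for setting a new checkpoint, teleporting to it and setting a temporary one, the last being an empty stub.
; Teleporting reopens the world level with the stored tag as the options string, intended to select the checkpoint's Player Start over the first one.
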(event `self.ReceiveBeginPlay`
  (add `self.Set-New-Checkpoint` (delegate `Set-New-Checkpoint_Event`))
  (add `self.Teleport-to-Checkpoint` (delegate `Teleport-to-Checkpoint_Event`))
  (add `self.Set-Temp-Checkpoint` (delegate `Set-Temp-Checkpoint_Event`)))

(event `Set-Temp-Checkpoint_Event`)

(event `Set-New-Checkpoint_Event` :!signature `self.Set-New-Checkpoint`
  (params (NewParam :type Boolean) (`String-Tag-Checkpoint` :type String))
  ;[0.9389 0 1 1 12] Setting the New Checkpoint.
  (bind _output_get (set `self.Tag-Checkpoint` `String-Tag-Checkpoint`))
  (`KismetSystemLibrary.PrintString` (`KismetStringLibrary.Concat_StrStr` "The new Checkpoint is " _output_get " \n---") true true (struct :`R` 1.0 :`G` 0.700438 :`A` 1.0)))

(event `Teleport-to-Checkpoint_Event`
  (bind _tag_checkpoint (`self.Tag-Checkpoint`))
  ;[0 1 0.4646 1 12] Reloading the Game Level, with the Checkpoint Player Start instead of the First Player Start
  (`KismetSystemLibrary.PrintString` (`KismetStringLibrary.Concat_StrStr` "Current Selected Checkpoint is " _tag_checkpoint " \n--") true true (struct :`R` 1.0 :`B` 0.75 :`A` 1.0))
  (`GameplayStatics.OpenLevelBySoftObjectPtr` (`self.World-Level-Name`) false _tag_checkpoint))