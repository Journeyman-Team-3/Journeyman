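; Camera_Dynamic is an actor that follows the player character from an elevated, diagonal angle.
; Each tick it caches the first player character's last movement update location, then calls CentreOnPlayer.
; That function places the actor at a configurable XY offset and fixed height above the player, rotating it to look at them, with no sweep or smoothing.
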(event `self.ReceiveBeginPlay`
  (set `self.playerPos` (`CharacterMovementComponent.GetLastUpdateLocation` (`Character.CharacterMovement` (`GameplayStatics.GetPlayerCharacter` 0)))))

(event `self.ReceiveTick`
  (params (DeltaSeconds :type "Float (single-precision)"))
  (set `self.playerPos` (`CharacterMovementComponent.GetLastUpdateLocation` (`Character.CharacterMovement` (`GameplayStatics.GetPlayerCharacter` 0))))
  (`self.CentreOnPlayer`))

(fn `CentreOnPlayer`
  (bind (_playerpos_x _playerpos_y _playerpos_z) (`KismetMathLibrary.BreakVector` (`self.playerPos`)))
  (bind _playercameraxy_offset (`self.playerCameraXY_Offset`))
  (bind _returnvalue (`KismetMathLibrary.MakeVector` (- _playerpos_x _playercameraxy_offset) (+ _playerpos_y _playercameraxy_offset) (+ _playerpos_z 5670.0)))
  (`self.K2_SetActorTransform` (`KismetMathLibrary.MakeTransform` _returnvalue (`KismetMathLibrary.FindLookAtRotation` _returnvalue (`self.playerPos`)))))

(fn `UserConstructionScript`)