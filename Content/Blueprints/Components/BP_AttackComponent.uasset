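; BP_AttackComponent is an unfinished attack component for Characters: SwingAttack, Tick and Range are all empty.
; Disconnected logic builds a temporary tagged rig on the owner, with a hidden cube pivot carrying an offset capsule and cube.
; A second disconnected chain yaws that pivot by RotationSpeed while IsSwinging until CurrentRotation reaches 180, then resets the counter and loops over tagged components without removing them.
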(event `Swing Attack`)

(event `self.ReceiveTick`
  (params (DeltaSeconds :type "Float (single-precision)")))

(fn `Range`)