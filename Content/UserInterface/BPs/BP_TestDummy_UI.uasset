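; Test dummy actor for enemy UI, with FocusOverlay, HPBar and FocusPrompt components.
; The construction script uses LockOn to show either the focus prompt alone (when true) or the focus overlay and HP bar (when false).
; On BeginPlay it copies GamepadModeOn into the EnemyFocusPrompt widget's GamepadMode and prints the value.
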(event `self.ReceiveBeginPlay`
  (`parent.ReceiveBeginPlay`)
  (bind _asenemy_focus_prompt (cast `/Game/UserInterface/UICompenents/EnemyFocusPrompt` (`WidgetComponent.GetWidget` (`self.FocusPrompt`))))
  (bind _output_get (set `/Game/UserInterface/UICompenents/EnemyFocusPrompt.GamepadMode` (`self.GamepadModeOn`) _asenemy_focus_prompt))
  (`KismetSystemLibrary.PrintString` (`KismetStringLibrary.Conv_BoolToString` _output_get)))

(fn `UserConstructionScript`
  (bind _focusoverlay (`self.FocusOverlay`))
  (bind _focusprompt (`self.FocusPrompt`))
  (`parent.UserConstructionScript`)
  (if (`self.LockOn`)
    (`SceneComponent.SetVisibility` _focusoverlay false false)
    (`SceneComponent.SetVisibility` (`self.HPBar`) false false)
    (`SceneComponent.SetVisibility` _focusprompt true false)
    (else
      (`SceneComponent.SetVisibility` _focusoverlay true false)
      (`SceneComponent.SetVisibility` (`self.HPBar`) true false)
      (`SceneComponent.SetVisibility` _focusprompt false false))))