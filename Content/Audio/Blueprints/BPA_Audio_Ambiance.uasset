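; Ambient audio actor that plays one of several music tracks at its location, covering idle and combat Woodlands and Cave themes plus a slime boss cue.
; On BeginPlay it binds play and stop dispatchers, selects the track by integer index, then fires the play dispatcher.
; Playback uses the audio player component's volume setting and an audio curve source's attenuation.
; The stop event only clears the sound reference, intended for exiting to main menu.
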(event `CustomEvent_0`
  (bind _info_audio_settings_volumemultiplier (break `/Game/Audio/Blueprints/Struct-Audio-Settings` (`/Game/Audio/Audio_Components/Blueprint_Componenets/Player_Character/BPC_Audio_Player.Info-Audio-Settings` (`self.BPC_Audio_Player`))))
  ;[1 1 1 1 10] Play sound at Actor Location with the current Sound Attenuation
  ; settings
  (`GameplayStatics.PlaySoundAtLocation` (`self.sfx-ambiance`) (`self.K2_GetActorLocation`) (struct) _info_audio_settings_volumemultiplier 1.0 0.0 (`AudioComponent.AttenuationSettings` (`self.AudioCurveSource`)) null null))

(event `Stop-Playing-Sfx`
  ;[1 1 1 1 10] Stopping the Editor from playing the Sfx, will be used when the player exits the gameto main menu.
  (set `self.sfx-ambiance` null))

(event `self.ReceiveBeginPlay`
  (`|ExecutionSequence`
    (:`then_0`
      ;[1 1 1 1 10] Play sound at Actor Location with the current Sound Attenuation
      ; settings
      (add `self.Play-Sfx` (delegate `CustomEvent_0`))
      ;[1 1 1 1 10] Stopping the Editor from playing the Sfx, will be used when the player exits the gameto main menu.
      (add `self.Stop-Sfx-Play` (delegate `Stop-Playing-Sfx`)))
    (:`then_1`
      (switch `int` (`self.Int-Select-Sfx`)
        (:`0`
          (set `self.sfx-ambiance` "/Game/Audio/Sound_Cues/Music/music-Idle-Woodlands.music-Idle-Woodlands"))
        (:`1`
          (set `self.sfx-ambiance` "/Game/Audio/Sound_Cues/Music/music-Combat-Woodlands.music-Combat-Woodlands"))
        (:`2`
          (set `self.sfx-ambiance` "/Game/Audio/Sound_Cues/Music/music-Idle-Cave.music-Idle-Cave"))
        (:`3`
          (set `self.sfx-ambiance` "/Game/Audio/Sound_Cues/Music/music-Combat-Cave.music-Combat-Cave"))
        (:`4`
          (set `self.sfx-ambiance` "/Game/Audio/Sound_Cues/Music/Boss-Music/Slime-Boss/sfx-cue-music-slime-boss.sfx-cue-music-slime-boss")))
      (`self.Play-Sfx`))))

(fn `UserConstructionScript`)