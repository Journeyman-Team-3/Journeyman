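; Actor component that manages the game's Master, Music, Effects and Ambient volume settings.
; On BeginPlay it sets MixMaster as the base sound mix and binds handlers to its two event dispatchers.
; The set-settings handler writes a new value into an index-keyed float array, then calls the assign dispatcher.
; The assign handler reapplies every array entry as a sound mix class override, debug-printing the music volume.
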(event `self.ReceiveBeginPlay`
  (`GameplayStatics.SetBaseSoundMix` "/Game/Audio/Sound-Mixers/Mix-Master.Mix-Master")
  (add `self.Set_New_Settings` (delegate `Set_New_Settings_Event`))
  (add `self.Assign_to_Sound_Class` (delegate `Assign_to_Sound_Class_Event`)))

(event `Assign_to_Sound_Class_Event`
  ;[0 0.2895 1 1 12] Assigning the Values of the Audio Settings to the Sound Classes
  (for (_array_element _array_index) (`self.Float_Audio_Settings`)
    (switch `int` _array_index
      (:`0`
        (`GameplayStatics.SetSoundMixClassOverride` "/Game/Audio/Sound-Mixers/Mix-Master.Mix-Master" "/Game/Audio/Sound-Class/SC-Master.SC-Master" _array_element) ; Master Sound Class
      )
      (:`1`
        (`GameplayStatics.SetSoundMixClassOverride` "/Game/Audio/Sound-Mixers/Mix-Master.Mix-Master" "/Game/Audio/Sound-Class/SC_Music.SC_Music" _array_element) ; Music Sound Class
        (`KismetSystemLibrary.PrintString` (`KismetStringLibrary.Concat_StrStr` "New Volume is set at: " (`KismetStringLibrary.Conv_DoubleToString` _array_element)) true true (struct :`R` 1.0 :`G` 0.64433 :`A` 1.0)))
      (:`2`
        (`GameplayStatics.SetSoundMixClassOverride` "/Game/Audio/Sound-Mixers/Mix-Master.Mix-Master" "/Game/Audio/Sound-Class/SC_Effects.SC_Effects" _array_element) ; Effects Sound Class
      )
      (:`3`
        (`GameplayStatics.SetSoundMixClassOverride` "/Game/Audio/Sound-Mixers/Mix-Master.Mix-Master" "/Game/Audio/Sound-Class/SC_Ambient.SC_Ambient" _array_element) ; Ambient Sound Class.
      ))))

(event `Set_New_Settings_Event` :!signature `self.Set_New_Settings`
  (params (New_Value :type "Float (double-precision)") (Int_Audio_Index :type Integer))
  ;[0.009193 0.3698 0 1 12] Setting the Audio Setting within the Array.
  (switch `int` Int_Audio_Index ; Switching on Int for determined Audio Setting:\n[0] = Master Volume (Currently not Working)\n[1] = Music Volume (Working and Assigned)\n[2] = Effects Volume (Working and Assigned)\n[3] = Ambient Volume (Working but Not Assigned).
    (:`0`
      (`KismetArrayLibrary.Array_Set` (`self.Float_Audio_Settings`) 0 New_Value))
    (:`1`
      (`KismetArrayLibrary.Array_Set` (`self.Float_Audio_Settings`) 1 New_Value))
    (:`2`
      (`KismetArrayLibrary.Array_Set` (`self.Float_Audio_Settings`) 2 New_Value))
    (:`3`
      (`KismetArrayLibrary.Array_Set` (`self.Float_Audio_Settings`) 3 New_Value)))
  (`self.Assign_to_Sound_Class`) ; Calling the Event Dispatcher that assigns the\nnew volume settings into the sound classes
)