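; Audio player component that selects combat sound effects (melee and block variants) and plays them at a given player location.
; On BeginPlay it binds its handlers to separate select-SFX and play-SFX events.
; Each select event stores the next of six InfoAudio sounds through a wrapping integer switch, so selection cycles in fixed order.
; The play event plays the currently stored sound at the supplied location.
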(event `self.ReceiveBeginPlay`
  (`|ExecutionSequence`
    (:`then_0`
      (add `self.Select_SFX` (delegate `SFX_Active`))
      (add `self.Play_SFX` (delegate `Play_Audio`)))))

(event `Play_Audio` :!signature `self.Play_SFX`
  (params (Player_Location :type "Vector Structure"))
  (`GameplayStatics.PlaySoundAtLocation` (`self.SFX_Selected_Audio`) Player_Location (struct) 1.0 1.0 0.0 null null null))

(event `SFX_Active`
  (bind (_info_audio_sfx_melee_empty _info_audio_sfx_melee_slime _info_audio_sfx_melee_skeleton _info_audio_sfx_melee_fox _info_audio_sfx_block_normal _info_audio_sfx_block_magical) (break `/Game/Audio/Components/Struct_Audio_Player` (`self.Info_Audio`)))
  (switch `int` (`self.int-switcher`)
    (:`0`
      (set `self.SFX_Selected_Audio` _info_audio_sfx_melee_empty)
      (`/Engine/EditorBlueprintResources/StandardMacros.IncrementInt` (`self.int-switcher`)))
    (:`1`
      (set `self.SFX_Selected_Audio` _info_audio_sfx_melee_slime)
      (`/Engine/EditorBlueprintResources/StandardMacros.IncrementInt` (`self.int-switcher`)))
    (:`2`
      (set `self.SFX_Selected_Audio` _info_audio_sfx_melee_skeleton)
      (`/Engine/EditorBlueprintResources/StandardMacros.IncrementInt` (`self.int-switcher`)))
    (:`3`
      (set `self.SFX_Selected_Audio` _info_audio_sfx_melee_fox)
      (`/Engine/EditorBlueprintResources/StandardMacros.IncrementInt` (`self.int-switcher`)))
    (:`4`
      (set `self.SFX_Selected_Audio` _info_audio_sfx_block_normal)
      (`/Engine/EditorBlueprintResources/StandardMacros.IncrementInt` (`self.int-switcher`)))
    (:`5`
      (set `self.SFX_Selected_Audio` _info_audio_sfx_block_magical)
      (set `self.int-switcher` 0))))