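; Audio component for enemy characters that supplies movement and hit sounds by enemy type.
; On BeginPlay it binds to dispatchers for enemy type, move and hit events.
; The type event copies Slime, Skeleton or Fox sounds from InfoSfxData, while Tree and Mimic get none.
; Both playback events currently play the move sound at world origin, so the hit sound goes unused despite comments indicating actor location.
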(event `self.ReceiveBeginPlay`
  (`|ExecutionSequence`
    (:`then_1`
      ;[0 0.1454 1 1 10] Binding Events to Event Dispatchers
      (add `self.Get_Type_of_Enemy` (delegate `Enemy_Type`))
      (add `self.Play_Sfx_Move` (delegate `Play_Move_Sfx`))
      (add `self.Play_Sfx_Hit` (delegate `Play_Hit_Sfx`)))))

(event `Play_Hit_Sfx`
  ;[1 1 1 1 10] SFX of the Enemy being Hit, Play at Actor Location...
  (`GameplayStatics.PlaySoundAtLocation` (`self.sfx_Move`) (0.0 0.0 0.0) (struct) 1.0 1.0 0.0 null null null))

(event `Play_Move_Sfx`
  ;[1 1 1 1 10] SFX of the Enemy Moving, Play at Actor Location...
  (`GameplayStatics.PlaySoundAtLocation` (`self.sfx_Move`) (0.0 0.0 0.0) (struct) 1.0 1.0 0.0 null null null))

(event `Enemy_Type`
  (params (int_Enemy_Type :type Integer))
  (bind (_info_sfx_data_sfx_slime_move _info_sfx_data_sfx_slime_jump _info_sfx_data_sfx_slime_hit _info_sfx_data_sfx_skeleton_move _info_sfx_data_sfx_skeleton_hit _info_sfx_data_sfx_fox_move _info_sfx_data_sfx_fox_hit) (break `/Game/Audio/Components/Struct_Audio_Enemy_Character` (`self.Info_Sfx_Data`)))
  (bind (_info_sfx_data_sfx_slime_move_2 _info_sfx_data_sfx_slime_jump_2 _info_sfx_data_sfx_slime_hit_2) (break `/Game/Audio/Components/Struct_Audio_Enemy_Character` (`self.Info_Sfx_Data`)))
  (bind (_info_sfx_data_sfx_slime_move_3 _info_sfx_data_sfx_slime_jump_3 _info_sfx_data_sfx_slime_hit_3 _info_sfx_data_sfx_skeleton_move_2 _info_sfx_data_sfx_skeleton_hit_2) (break `/Game/Audio/Components/Struct_Audio_Enemy_Character` (`self.Info_Sfx_Data`)))
  ;[0.9708 0 1 1 10] Assigning the Corrosponding SFXs to the Enemy Types.
  (switch `int` int_Enemy_Type
    (:`0`
      ;;[1 1 1 1 10] Assigning the Slime SFXs...
      (`KismetSystemLibrary.PrintString` "Enemy is a Slime")
      (set `self.sfx_Move` _info_sfx_data_sfx_slime_move_2)
      (set `self.sfx_Hit` _info_sfx_data_sfx_slime_hit_2))
    (:`1`
      ;;[1 1 1 1 10] Assigning the Skeleton SFXs...
      (`KismetSystemLibrary.PrintString` "Enemy is a Skeleton")
      (set `self.sfx_Move` _info_sfx_data_sfx_skeleton_move_2)
      (set `self.sfx_Hit` _info_sfx_data_sfx_skeleton_hit_2))
    (:`2`
      ;;[1 1 1 1 10] Assigning the Fox SFXs...
      (`KismetSystemLibrary.PrintString` "Enemy is a Fox")
      (set `self.sfx_Move` _info_sfx_data_sfx_fox_move)
      (set `self.sfx_Hit` _info_sfx_data_sfx_fox_hit))
    (:`3`
      ;;[1 1 1 1 10] Assigning the Tree SFXs...
      (`KismetSystemLibrary.PrintString` "Enemy is a Tree")
      (set `self.sfx_Move` null)
      (set `self.sfx_Hit` null))
    (:`4`
      ;;[1 1 1 1 10] Assigning the Mimic SFXs...
      (`KismetSystemLibrary.PrintString` "Enemy is a Mimic")
      (set `self.sfx_Move` null)
      (set `self.sfx_Hit` null))))