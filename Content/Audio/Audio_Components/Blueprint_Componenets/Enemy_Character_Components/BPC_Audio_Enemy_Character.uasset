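; Audio component for enemy characters that plays their idle, move, hit and interaction sound effects in the world.
; On BeginPlay it binds one custom event to each of the four matching SFX event dispatchers.
; When a dispatcher fires, its event plays the corresponding sound variable at the location passed in, keeping playback decoupled from whatever triggers it.
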(event `self.ReceiveBeginPlay`
  (`|ExecutionSequence`
    (:`then_1`
      ;[0 0.1454 1 1 10] Binding Events to Event Dispatchers
      (add `self.Play_Sfx_Idle` (delegate `Play_Idle_Sfx`))
      (add `self.Play_Sfx_Move` (delegate `Play_Move_Sfx`))
      (add `self.Play_Sfx_Hit` (delegate `Play_Hit_Sfx`))
      (add `self.Play_Sfx_Interaction` (delegate `Play_Interaction`)))))

(event `Play_Idle_Sfx` :!signature `self.Play_Sfx_Idle`
  (params (Location :type "Vector Structure"))
  ;[0 0.67 1 1 10] Playing the idle sfx at desired location.
  (`GameplayStatics.PlaySoundAtLocation` (`self.sfx_Idle`) Location (struct) 1.0 1.0 0.0 null null null))

(event `Play_Interaction` :!signature `self.Play_Sfx_Interaction`
  (params (Location :type "Vector Structure"))
  ;[0 0.67 1 1 10] Play Unique Sound at Location
  (`GameplayStatics.PlaySoundAtLocation` (`self.sfx_Interaction`) Location (struct) 1.0 1.0 0.0 null null null))

(event `Play_Move_Sfx` :!signature `self.Play_Sfx_Move`
  (params (Location :type "Vector Structure"))
  ;[0 0.67 1 1 10] SFX of the Enemy Moving, Play at Actor Location...
  (`GameplayStatics.PlaySoundAtLocation` (`self.sfx_Move`) Location (struct) 1.0 1.0 0.0 null null null))

(event `Play_Hit_Sfx` :!signature `self.Play_Sfx_Hit`
  (params (Location :type "Vector Structure"))
  ;[0 0.67 1 1 10] SFX of the Enemy being Hit, Play at Actor Location...
  (`GameplayStatics.PlaySoundAtLocation` (`self.sfx_Hit`) Location (struct) 1.0 1.0 0.0 null null null))