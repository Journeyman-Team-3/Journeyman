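; Rotatable grinder puzzle piece that feeds the Graveyard_Puzzle_Gate counter.
; While the player stands in either of two boxes, Tick yaws Cylinder2 in that box's direction, with Box taking priority.
; Each step compares rotation to TargetAngle within Variance; when outside tolerance, it adds Point to the gate's Current, then zeroes Point.
; Debug prints show rotation and gate count.
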(event `self.ReceiveTick`
  (params (DeltaSeconds :type "Float (single-precision)"))
  (bind _relativerotation (`SceneComponent.RelativeRotation` (`self.Cylinder2`)))
  (if (`self.overlappingBox`)
    ;[1 1 1] Rotate in minus dir
    (if (`PrimitiveComponent.IsOverlappingActor` (`self.Box`) (`GameplayStatics.GetPlayerPawn` 0))
      (`SceneComponent.K2_AddLocalRotation` (`self.Cylinder2`) (* (`KismetMathLibrary.MakeRotator` 0.0 0.0 (`self.RotationSpeed`)) -1.0) false false)
      (`KismetSystemLibrary.PrintString` (`KismetStringLibrary.Concat_StrStr` "Box: " (`KismetStringLibrary.Conv_RotatorToString` (`SceneComponent.RelativeRotation` (`self.Cylinder2`)))))
      ;[1 1 1] When rotated to correct place, increase gate value +1, if moved out of place return gate value by -1
      (set `self.CurrentRotation` _relativerotation :!label _label)
      (bind _output_get (set `self.IsAngled` (== (`self.CurrentRotation`) (`self.Target_Angle`) :`ErrorTolerance` (`self.Variance`))))
      (if (not _output_get)
        (`KismetSystemLibrary.PrintString` (`KismetStringLibrary.Concat_StrStr` "Correct is: " (`KismetStringLibrary.Conv_BoolToString` _output_get)) true true (struct :`R` 1.0 :`B` 0.046772 :`A` 1.0))
        (bind _returnvalue (`GameplayStatics.GetActorOfClass` "/Game/PersonalFolders/Cali/Graveyard_Puzzle_Gate.Graveyard_Puzzle_Gate_C"))
        (bind _asgraveyard_puzzle_gate (cast `/Game/PersonalFolders/Cali/Graveyard_Puzzle_Gate` _returnvalue))
        (bind _output_get_2 (set `/Game/PersonalFolders/Cali/Graveyard_Puzzle_Gate.Current` (+ (`/Game/PersonalFolders/Cali/Graveyard_Puzzle_Gate.Current` _asgraveyard_puzzle_gate) (`self.Point`)) _asgraveyard_puzzle_gate))
        (set `self.Point` 0)
        (`KismetSystemLibrary.PrintString` (`KismetStringLibrary.Conv_IntToString` _output_get_2) true true (struct :`R` 0.996819 :`B` 1.0 :`A` 1.0)))
      (else
        (set `self.overlappingBox` false)))
    (else
      ;[1 1 1] else check if Overlapping other box THEN rotate
      (if (`self.overlappingBox1`)
        (if (`PrimitiveComponent.IsOverlappingActor` (`self.Box1`) (`GameplayStatics.GetPlayerPawn` 0))
          (`SceneComponent.K2_AddLocalRotation` (`self.Cylinder2`) (* (`KismetMathLibrary.MakeRotator` 0.0 0.0 (`self.RotationSpeed`)) 1.0) false false)
          (`KismetSystemLibrary.PrintString` (`KismetStringLibrary.Concat_StrStr` "Box1:  " (`KismetStringLibrary.Conv_RotatorToString` _relativerotation)))
          (goto _label)
          (else
            (set `self.overlappingBox1` false)))))))

(event `self.Box.OnComponentBeginOverlap`
  (params (OverlappedComponent :type "PrimitiveComponent Object Reference") (OtherActor :type "Actor Object Reference") (OtherComp :type "PrimitiveComponent Object Reference") (OtherBodyIndex :type Integer) (bFromSweep :type Boolean) (SweepResult :type "HitResult Structure (by ref)"))
  (set `self.overlappingBox` true))

(event `self.Box1.OnComponentBeginOverlap`
  (params (OverlappedComponent :type "PrimitiveComponent Object Reference") (OtherActor :type "Actor Object Reference") (OtherComp :type "PrimitiveComponent Object Reference") (OtherBodyIndex :type Integer) (bFromSweep :type Boolean) (SweepResult :type "HitResult Structure (by ref)"))
  (set `self.overlappingBox1` true))

(fn `UserConstructionScript`)