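; Scene capture actor that follows the player and captures only components tagged GrassAffector, likely to drive grass interaction in materials.
; On BeginPlay it adds tagged components of tagged actors to the capture's show-only list and publishes its ortho width as CaptureSize.
; Each tick MoveCapture places it just above player 0 and writes CaptureLocation to the Noah_Global_Mat_Params collection.
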(event `self.ReceiveBeginPlay`
  (`KismetMaterialLibrary.SetScalarParameterValue` "/Game/PersonalFolders/Noah/Materials/Noah_Global_Mat_Params.Noah_Global_Mat_Params" "CaptureSize" (`SceneCaptureComponent2D.OrthoWidth` (`self.SceneCapture`)))
  (bind _outactors (`GameplayStatics.GetAllActorsWithTag` "GrassAffector"))
  (for _array_element _outactors
    (for _array_element_2 (`self.GetComponentsByTag` _array_element "/Script/Engine.PrimitiveComponent" "GrassAffector")
      (`SceneCaptureComponent.ShowOnlyComponent` (`self.SceneCapture`) _array_element_2))))

(event `self.ReceiveTick`
  (params (DeltaSeconds :type "Float (single-precision)"))
  (`self.MoveCapture`))

(fn `MoveCapture`
  (bind (_returnvalue_x _returnvalue_y _returnvalue_z) (`KismetMathLibrary.BreakVector` (`self.K2_GetActorLocation` (`GameplayStatics.GetPlayerCharacter` 0))))
  (`self.K2_SetActorLocation` (`KismetMathLibrary.MakeVector` _returnvalue_x _returnvalue_y (+ _returnvalue_z 100.0)))
  (`KismetMaterialLibrary.SetVectorParameterValue` "/Game/PersonalFolders/Noah/Materials/Noah_Global_Mat_Params.Noah_Global_Mat_Params" "CaptureLocation" (`KismetMathLibrary.Conv_VectorToLinearColor` (`self.K2_GetActorLocation`))))

(fn `SetCaptureSize`
  (`KismetMaterialLibrary.SetScalarParameterValue` "/Game/PersonalFolders/Noah/Materials/Noah_Global_Mat_Params.Noah_Global_Mat_Params" "CaptureSize" (`SceneCaptureComponent2D.OrthoWidth` (`self.SceneCapture`))))

(fn `UserConstructionScript`)